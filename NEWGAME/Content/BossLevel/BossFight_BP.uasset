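; Boss tank for the boss level that moves via a BossFight routine, hunts the player and fires physics-launched RPG rounds.
; Tick line-traces for the player, raising or lowering an alert level that halts movement to track them; full alert arms a polling Delay loop that fires and resets.
; Damage, including box overlaps, updates a health bar; death triggers explosion, fire and narration, then returns to the main menu.
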(event OnComponentBeginOverlap(Box)
  (params (OverlappedComponent :type Primitive%20Component%20Object%20Reference) (OtherActor :type Actor%20Object%20Reference) (OtherComp :type Primitive%20Component%20Object%20Reference) (OtherBodyIndex :type Integer) (bFromSweep :type Boolean) (SweepResult :type Hit%20Result%20Structure%20%28by%20ref%29))
  (Game|Damage|ApplyDamage self 2e+02 0 0))

(event OnComponentBeginOverlap(Box1)
  (params (OverlappedComponent :type Primitive%20Component%20Object%20Reference) (OtherActor :type Actor%20Object%20Reference) (OtherComp :type Primitive%20Component%20Object%20Reference) (OtherBodyIndex :type Integer) (bFromSweep :type Boolean) (SweepResult :type Hit%20Result%20Structure%20%28by%20ref%29))
  (Game|Damage|ApplyDamage self 2e+02 0 0))

(event EventBeginPlay
  (if (> (Variables|Default|GetCurrentHealth) 0.0)
    (Utilities|FlowControl|Sequence
      (:then_0
        ;[0.15 0.15 0.15 0.5] Will Shoot and then continue moving if the player is already not in sight
        (if (Variables|Default|GetAlarmOn) :!label _label
          (CallFunction|Fire (Transformation|GetActorLocation (stale EventTick _detectedactor)))
          (Variables|Default|SetAlarmOn false)
          (Variables|Default|SetAlertLevel 0.0)
          (Variables|Default|SetMove true)
          (Utilities|FlowControl|Delay 5.0)
          (goto _label)
          (else
            (Utilities|FlowControl|Delay 0.2)
            (goto _label))))
      (:then_1
        (bind _returnvalue (UserInterface|CreateWidget "/Game/BossLevel/WBP_HealthBar.WBP_HealthBar_C"))
        (UserInterface|Viewport|AddtoViewport _returnvalue 0)
        (Default|Initalise _returnvalue self))
      (:then_2
        (Audio|PlaySoundatLocation "/Game/ImportAudio/Sports-car-engine-driving-loopable-460.Sports-car-engine-driving-loopable-460" (Transformation|GetActorLocation) "0, 0, 0" 0.2 1.0 0.0 "/Game/ImportAudio/BigSound.BigSound" 0 0 0)))))

(event EventTick
  (params (DeltaSeconds :type Float%20%28single-precision%29))
  (if (not (Variables|Default|GetDead?))
    (Utilities|FlowControl|Sequence
      (:then_0
        ;[0.15 0.15 0.15 0.5] Moves the Turret around and arround
        (Class|BossMovement|BossFight self (Variables|Default|GetMove) DeltaSeconds))
      (:then_1
        ;[0.15 0.15 0.15 0.5] Searches and Detects a player
        (bind _detectedactor (Class|PhysicsChecker|LineTrace (Variables|Default|GetFirePoint) 5e+03 4e+01 false))
        (Utilities|Casting|CastToBP_FPS_CharacterGun _detectedactor
          (:then
            (CallFunction|IncreaseAlert))
          (:CastFailed
            (CallFunction|DecreaseAlert))))
      (:then_2
        ;[0.15 0.15 0.15 0.5] This when the Tank first sees the player will follow the player until it shoots or the player hides
        (if (> (Variables|Default|GetAlertLevel) 0.0)
          (Variables|Default|SetMove false)
          (Class|BossMovement|LookatPlayer self _detectedactor)
          (else
            (Variables|Default|SetMove true)))))))

(event Game|Damage|EventAnyDamage
  (params (Damage :type Float%20%28single-precision%29) (DamageType :type Damage%20Type%20Object%20Reference) (InstigatedBy :type Controller%20Object%20Reference) (DamageCauser :type Actor%20Object%20Reference))
  (bind _output_get (Variables|Default|SetCurrentHealth (- (Variables|Default|GetCurrentHealth) Damage)))
  (Default|CallEHealthUpdated _output_get (Variables|Default|GetMaxHealth))
  (if (<= (Variables|Default|GetCurrentHealth) 0.0)
    (Effects|SpawnEmitteratLocation "/Game/StarterContent/Particles/P_Explosion.P_Explosion" (Transformation|GetActorLocation self) "0, 0, 0" "20.000000,20.000000,20.000000")
    (Variables|Default|SetDead? true)
    (Effects|SpawnEmitteratLocation "/Game/StarterContent/Particles/P_Fire.P_Fire" (Transformation|GetWorldLocation (Variables|Default|GetBox)) "0, 0, 0" "10.000000,10.000000,10.000000")
    (Audio|PlaySound2D "/Game/ImportAudio/Narrator6.Narrator6" 0.4 0.95 0.0 0 0)
    (Utilities|FlowControl|Delay 7.0)
    (Game|OpenLevel(byName) "MainMenu")))

(event EventTakeHit
  (params (Inverse%20Impact%20Normal :type Vector :default "0, 0, 0"))
  (Game|Damage|ApplyDamage self 1.0 0 0))

(fn ConstructionScript)

(fn DecreaseAlert
  (Variables|Default|SetAlertLevel (Math|Float|Clamp(Float) (- (Variables|Default|GetAlertLevel) (Variables|Default|GetAlertStepDown)) 0.0 (Variables|Default|GetAlertTarget)))
  (if (<= (Variables|Default|GetAlertLevel) (Variables|Default|GetAlertReleaseThreshold))
    (Variables|Default|SetAlarmOn false)))

(fn IncreaseAlert
  (Variables|Default|SetAlertLevel (Math|Float|Clamp(Float) (+ (Variables|Default|GetAlertLevel) (Variables|Default|GetAlertStepUp)) 0.0 (Variables|Default|GetAlertTarget)))
  (if (>= (Variables|Default|GetAlertLevel) (Variables|Default|GetAlertTarget))
    (Variables|Default|SetAlarmOn true)))

(fn Fire
  (params (RotationLook :type Vector))
  (Audio|PlaySoundatLocation "/Game/ImportAudio/Armored-tank-cannon-fire-single-shot-288.Armored-tank-cannon-fire-single-shot-288" (Transformation|GetActorLocation) "0, 0, 0" 1.0 1.0 0.0 "/Game/ImportAudio/BigSound.BigSound" 0 0 0)
  (bind _returnvalue (Game|SpawnActorfromClass "/Game/BossLevel/RPG_BP_AMM.RPG_BP_AMM_C" (Transformation|GetWorldTransform (Variables|Default|GetFirePoint2)) "Undefined" "MultiplyWithRoot" 0 0))
  (CallFunction|Impulse _returnvalue RotationLook))

(fn Impulse
  (params (NewParam :type RPG%20BP%20AMM%20Object%20Reference) (RotationLook :type Vector))
  (Physics|SetPhysicsLinearVelocity (Variables|/Game/BossLevel/RPG_BP_AMM.RPG_BP_AMM_C|Getrpg71 NewParam) (* (Math|Vector|GetForwardVector (Variables|Default|GetFirePoint2)) (Variables|Default|GetBulletVelocity)) false "None"))