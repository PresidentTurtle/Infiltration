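; AI enemy character for the boss level that plays footsteps while moving and melee-attacks overlapping actors.
; An overlap starts the attack montage, then deals damage after a short delay unless the enemy is already ragdolled.
; The first TakeHit ragdolls body and bat, sets the blackboard Dead key and plays a random death sound; later hits push the ragdoll.
; After a delay it destroys itself and calls SpawnActor at its starting transform.
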(event EventBeginPlay
  (bind _sound (Variables|Default|GetSound))
  (Variables|Default|SetTransform (Transformation|GetActorTransform))
  (if (> (Math|Vector|VectorLength (Transformation|GetVelocity)) 0.0) :!label _label
    (Audio|PlaySoundatLocation (Utilities|Array|Get(acopy) _sound (Math|Random|RandomIntegerinRange 0 (- (Utilities|Array|Length _sound) 1))) (Transformation|GetActorLocation) "0, 0, 0" 0.1 1.0 0.0 "/Game/ImportAudio/LittleSound.LittleSound" 0 0 0)
    (Utilities|FlowControl|Delay 0.3)
    (goto _label)
    (else
      (Utilities|FlowControl|Delay 0.2)
      (goto _label))))

(event Collision|EventActorBeginOverlap
  (params (OtherActor :type Actor%20Object%20Reference))
  (Animation|PlayAnimMontage "/Game/Assets/Characters/Arms/Arms_Animations/Anim_Montages/Arms_Melee_Attack_Montage.Arms_Melee_Attack_Montage" 1.0 "None")
  (Utilities|FlowControl|Delay 0.3)
  (if (not (Variables|Default|GetPhysics))
    (Class|DamageTaken|DamageTake(Message) OtherActor 15)
    (Components|Animation|SetAnimationMode (Variables|Character|GetMesh) "AnimationBlueprint" true)))

(event EventTakeHit
  (params (Inverse%20Impact%20Normal :type Vector :default "0, 0, 0"))
  (bind _returnvalue (Class|KismetMathLibrary|RandomInteger64inRange 0 30))
  (if (Variables|Default|GetPhysics)
    (Physics|AddImpulse (Variables|Character|GetMesh) (* Inverse%20Impact%20Normal (Variables|Default|GetMultipler)) "None" false)
    (else
      (Physics|SetSimulatePhysics (Variables|Character|GetMesh) true)
      (Physics|SetSimulatePhysics (Variables|Default|GetSM_Survival_Character_Bat) true)
      (Components|Animation|SetAnimation (Variables|Character|GetMesh) 0)
      (AI|Components|Blackboard|SetValueasBool (AI|GetBlackboard 0) (Utilities|Name|MakeLiteralName "Dead") true)
      (Variables|Default|SetPhysics true)
      (if (> _returnvalue 10)
        (if (> _returnvalue 20)
          (Audio|PlaySoundatLocation "/Game/ImportAudio/Death-shout-anime-villain-vocalization-492.Death-shout-anime-villain-vocalization-492" (Transformation|GetActorLocation) "0, 0, 0" 0.1 1.0 0.0 "/Game/ImportAudio/BasicSound.BasicSound" 0 0 0)
          (else
            (Audio|PlaySoundatLocation "/Game/ImportAudio/Man-pain-ohh-671.Man-pain-ohh-671" (Transformation|GetActorLocation) "0, 0, 0" 0.1 1.0 0.0 "/Game/ImportAudio/BasicSound.BasicSound" 0 0 0)))
        (else
          (Audio|PlaySoundatLocation "/Game/ImportAudio/Death-scream-man-dying-pain-791.Death-scream-man-dying-pain-791" (Transformation|GetActorLocation) "0, 0, 0" 0.1 1.0 0.0 "/Game/ImportAudio/BasicSound.BasicSound" 0 0 0)))
      (Pawn|Components|CharacterMovement|DisableMovement (Variables|Character|GetCharacterMovement))
      (Utilities|FlowControl|Delay 4e+01)
      (Actor|DestroyActor)
      (Variables|Default|SetPhysics false)
      (if true
        (Game|SpawnActorfromClass "AI_Mechanic_BP_C" (Variables|Default|GetTransform) "Undefined" "OverrideRootScale" 0 0)))))

(fn ConstructionScript)