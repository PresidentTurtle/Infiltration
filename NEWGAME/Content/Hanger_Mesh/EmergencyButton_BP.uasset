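; Emergency button actor that switches a set of linked cameras through their OnOrOffMessage call.
; On BeginPlay it sends true to every entry in its Camera array and hides its prompt widget, which shows only while an actor overlaps it.
; Interact sends false to each camera and plays an attenuated click sound at the button, once per camera, with no path to switch them back.
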(event EventBeginPlay
  (Development|SetHiddeninGame (Variables|Default|GetWidget) true false)
  (for _array_element (Variables|Default|GetCamera)
    (Class|CameraonOff|OnorOff(Message) _array_element true)))

(event Collision|EventActorBeginOverlap
  (params (OtherActor :type Actor%20Object%20Reference))
  (Development|SetHiddeninGame (Variables|Default|GetWidget) false false))

(event EventTick
  (params (DeltaSeconds :type Float%20%28single-precision%29)))

(event Collision|EventActorEndOverlap
  (params (OtherActor :type Actor%20Object%20Reference))
  (Development|SetHiddeninGame (Variables|Default|GetWidget) true false))

(event EventInteract
  (for _array_element (Variables|Default|GetCamera)
    (Class|CameraonOff|OnorOff(Message) _array_element false)
    (Audio|PlaySoundatLocation "/Game/ImportAudio/Camping-flashlight-turning-on-and-off-412.Camping-flashlight-turning-on-and-off-412" (Transformation|GetActorLocation) "0, 0, 0" 0.1 1.0 0.0 "/Game/ImportAudio/BasicSound.BasicSound" 0 0 0)))

(fn ConstructionScript)