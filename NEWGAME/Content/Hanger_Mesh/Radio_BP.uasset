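; Radio prop actor for the hangar that the player can switch on and off through an Interact event.
; Overlapping the actor shows its widget, which is otherwise hidden.
; Switching toggles both audio components between muted and low volume rather than stopping them.
; Switching on plays Audio from the start and enters a Delay loop that periodically replays Radio2, which keeps running while muted.
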(event EventBeginPlay
  (Development|SetHiddeninGame (Variables|Default|GetWidget) true false)
  (Audio|Components|Audio|SetVolumeMultiplier (Variables|Default|GetAudio) 0.0 :!class /Script/Engine.AudioComponent)
  (Audio|Components|Audio|SetVolumeMultiplier (Variables|Default|GetRadio2) 0.0 :!class /Script/Engine.AudioComponent))

(event Collision|EventActorBeginOverlap
  (params (OtherActor :type Actor%20Object%20Reference))
  (Development|SetHiddeninGame (Variables|Default|GetWidget) false false))

(event Collision|EventActorEndOverlap
  (params (OtherActor :type Actor%20Object%20Reference))
  (Development|SetHiddeninGame (Variables|Default|GetWidget) true false))

(event EventInteract
  (if (Variables|Default|GetOn?)
    (Variables|Default|SetOn? false)
    (Audio|Components|Audio|SetVolumeMultiplier (Variables|Default|GetAudio) 0.0 :!class /Script/Engine.AudioComponent)
    (Audio|Components|Audio|SetVolumeMultiplier (Variables|Default|GetRadio2) 0.0 :!class /Script/Engine.AudioComponent)
    (else
      (Variables|Default|SetOn? true)
      (Audio|Components|Audio|SetVolumeMultiplier (Variables|Default|GetAudio) 0.2 :!class /Script/Engine.AudioComponent)
      (Audio|Components|Audio|SetVolumeMultiplier (Variables|Default|GetRadio2) 0.2 :!class /Script/Engine.AudioComponent)
      (Audio|Components|Audio|Play (Variables|Default|GetAudio) 0.0)
      (Utilities|FlowControl|Delay 5.0 :!label _label)
      (Audio|Components|Audio|Play (Variables|Default|GetRadio2) 0.0)
      (Utilities|FlowControl|Delay 2e+01)
      (goto _label))))

(fn ConstructionScript)