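; BuildingSound_BP is an actor that drives an Ambient audio component for a building through an "Inside" bool sound parameter.
; BeginPlay sets Inside to true and starts playback.
; Actor overlap begin sets Inside to false and overlap end sets it back to true, with no filter on the overlapping actor.
; Both overlap events also set the volume multiplier to zero before calling Play again, and nothing here restores it.
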(event EventBeginPlay
  (Effects|Components|ParticleSystem|SetBoolParameter (Variables|Default|GetAmbient) "Inside" true)
  (Audio|Components|Audio|Play (Variables|Default|GetAmbient) 0.0))

(event Collision|EventActorBeginOverlap
  (params (OtherActor :type Actor%20Object%20Reference))
  (Audio|Components|Audio|SetVolumeMultiplier (Variables|Default|GetAmbient) 0.0 :!class /Script/Engine.AudioComponent)
  (Effects|Components|ParticleSystem|SetBoolParameter (Variables|Default|GetAmbient) "Inside" false)
  (Audio|Components|Audio|Play (Variables|Default|GetAmbient) 0.0))

(event Collision|EventActorEndOverlap
  (params (OtherActor :type Actor%20Object%20Reference))
  (Audio|Components|Audio|SetVolumeMultiplier (Variables|Default|GetAmbient) 0.0 :!class /Script/Engine.AudioComponent)
  (Effects|Components|ParticleSystem|SetBoolParameter (Variables|Default|GetAmbient) "Inside" true)
  (Audio|Components|Audio|Play (Variables|Default|GetAmbient) 0.0))

(fn ConstructionScript)